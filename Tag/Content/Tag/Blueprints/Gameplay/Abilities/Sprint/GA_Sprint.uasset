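; Sprint gameplay ability that runs while input is held and the ability cost can be paid.
; Activation applies GE_Sprint and starts sprinting on the Tag character movement component; ending removes the effect and stops sprinting.
; A short delay loop with a server-wait net sync commits the cost only while the character accelerates on the ground.
; Input release or a failed cost commit ends the ability.
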(event `self.K2_ActivateAbility`
  (set `self.EndSprint` false)
  (bind _returnvalue (`self.BP_ApplyGameplayEffectToOwner` "/Game/Tag/Blueprints/Gameplay/Abilities/Sprint/GE_Sprint.GE_Sprint_C" (`self.GetAbilityLevel`)))
  (set `self.GESprint` _returnvalue)
  (bind _astag_character_movement_component (cast `TagCharacterMovementComponent` (`.MovementComponent` (break `GameplayAbilityActorInfo` (`self.GetActorInfo`)))))
  (`TagCharacterMovementComponent.StartSprinting` _astag_character_movement_component)
  (`AbilityTask_WaitInputRelease.WaitInputRelease` false
    (:`then`
      (`AbilityTask_WaitDelay.WaitDelay` 0.05 :!label _label
        (:`OnFinish`
          (`AbilityTask_NetworkSyncPoint.WaitNetSync` "OnlyServerWait"
            (:`then`
              (bind _ascharacter_movement_component (cast `CharacterMovementComponent` (`.MovementComponent` (break `GameplayAbilityActorInfo` (`self.GetActorInfo`)))))
              (if (and (> (`KismetMathLibrary.VSize` (`CharacterMovementComponent.GetCurrentAcceleration` _ascharacter_movement_component)) 0.0) (not (`NavMovementComponent.IsFalling` _ascharacter_movement_component)))
                (bind _returnvalue_2 (`self.K2_CommitAbilityCost` false))
                (if _returnvalue_2
                  (if (not (`self.EndSprint`)) :!label _label_2
                    (goto _label))
                  (else
                    (set `self.EndSprint` true :!label _label_3)
                    (`self.K2_EndAbility`)))
                (else
                  (goto _label_2))))))))
    (:`OnRelease`
      (goto _label_3))))

(event `self.K2_OnEndAbility`
  (params (bWasCancelled :type Boolean))
  (`self.BP_RemoveGameplayEffectFromOwnerWithHandle` (`self.GESprint`))
  (bind _astag_character_movement_component (cast `TagCharacterMovementComponent` (`.MovementComponent` (break `GameplayAbilityActorInfo` (`self.GetActorInfo`)))))
  (`TagCharacterMovementComponent.StopSprinting` _astag_character_movement_component))